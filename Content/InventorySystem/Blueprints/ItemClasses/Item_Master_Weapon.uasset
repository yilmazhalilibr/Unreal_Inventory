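; Master Blueprint class for weapon items in the inventory system, which equips the weapon on the character when used.
; On the onUsed event, it passes itself to EquipItem on the inventory's TapDownCharRef and destroys its actor if that call returns false.
; BeginPlay, overlap and Tick are disabled stubs, and the construction script only calls its parent.
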(event EventBeginPlay
  (|CallParentFunction) ; This node is disabled and will not be called.\nDrag off pins to build functionality.
)

(event Collision|EventActorBeginOverlap
  (params (OtherActor :type Actor%20Object%20Reference))
  (|CallParentFunction OtherActor) ; This node is disabled and will not be called.\nDrag off pins to build functionality.
)

(event EventTick
  (params (DeltaSeconds :type Float%20%28single-precision%29))
  (|CallParentFunction DeltaSeconds) ; This node is disabled and will not be called.\nDrag off pins to build functionality.
)

(event EventEventonUsed
  (params (Inventory :type BP%20Inventory%20Object%20Reference))
  (bind _success_ (Default|EquipItem (Variables|/Game/InventorySystem/Blueprints/BP_Inventory.BP_Inventory_C|GetTapDownCharRef Inventory) self))
  (if (not _success_)
    (Actor|DestroyActor)))

(fn ConstructionScript
  (|CallParentFunction))