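; Merchant actor that opens a shop for the top-down character.
; A sphere overlap toggles the merchant text; both begin and end assign the merchant as the character's NearbyMerchant, never clearing it.
; OnInteract, gated by a DoOnce, creates a centered shop widget, refreshes the inventory and stops player movement.
; OnShopClosed restores walking, refreshes any visible inventory, re-enables its widget, removes the shop and resets the gate.
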(event OnComponentBeginOverlap(Sphere)
  (params (OverlappedComponent :type Primitive%20Component%20Object%20Reference) (OtherActor :type Actor%20Object%20Reference) (OtherComp :type Primitive%20Component%20Object%20Reference) (OtherBodyIndex :type Integer) (bFromSweep :type Boolean) (SweepResult :type Hit%20Result%20Structure%20%28by%20ref%29))
  (bind _astop_down_character (Utilities|Casting|CastToTopDownCharacter OtherActor))
  (Variables|/Game/TopDownBP/Blueprints/TopDownCharacter.TopDownCharacter_C|SetNearbyMerchant _astop_down_character self)
  (Rendering|SetVisibility (Variables|Default|GetMerchantText) true false))

(event OnComponentEndOverlap(Sphere)
  (params (OverlappedComponent :type Primitive%20Component%20Object%20Reference) (OtherActor :type Actor%20Object%20Reference) (OtherComp :type Primitive%20Component%20Object%20Reference) (OtherBodyIndex :type Integer))
  (bind _astop_down_character (Utilities|Casting|CastToTopDownCharacter OtherActor))
  (Variables|/Game/TopDownBP/Blueprints/TopDownCharacter.TopDownCharacter_C|SetNearbyMerchant _astop_down_character self)
  (Rendering|SetVisibility (Variables|Default|GetMerchantText) false false))

(event Custom|OnInteract
  (params (TopDownChar :type Top%20Down%20Character%20Object%20Reference))
  (Utilities|FlowControl|DoOnce false
    (:Completed
      (bind _output_get (Variables|Default|SetTopDownCharRef TopDownChar))
      (bind _returnvalue (UserInterface|CreateWidget "/Game/InventorySystem/Widgets/ShopWidget.ShopWidget_C" 0 self _output_get))
      (bind _output_get_2 (Variables|Default|SetShopWidget _returnvalue))
      (Class|UserWidget|SetPositioninViewport _output_get_2 "(X=0.000000,Y=0.000000)" false)
      (Class|UserWidget|SetAnchorsinViewport _output_get_2 (Utilities|Struct|MakeAnchors "(X=0.500000,Y=0.500000)" "(X=0.500000,Y=0.500000)"))
      (Class|UserWidget|SetAlignmentinViewport _output_get_2 "(X=0.500000,Y=0.500000)")
      (UserInterface|Viewport|AddtoViewport _output_get_2 5)
      (Default|HideInventory (Variables|/Game/TopDownBP/Blueprints/TopDownCharacter.TopDownCharacter_C|GetInventoryRef (Variables|Default|GetTopDownCharRef)))
      (Default|ShowInventory (Variables|/Game/TopDownBP/Blueprints/TopDownCharacter.TopDownCharacter_C|GetInventoryRef (Variables|Default|GetTopDownCharRef)))
      (Variables|/Game/TopDownBP/Blueprints/TopDownCharacter.TopDownCharacter_C|SetIsShopOpen? (Variables|Default|GetTopDownCharRef) true)
      (Pawn|Components|CharacterMovement|DisableMovement (Variables|/Script/Engine.Character|GetCharacterMovement (Variables|Default|GetTopDownCharRef)))
      (Components|Movement|StopMovementImmediately (Variables|/Script/Engine.Character|GetCharacterMovement (Variables|Default|GetTopDownCharRef))))))

(event Custom|OnShopClosed
  (Variables|/Game/TopDownBP/Blueprints/TopDownCharacter.TopDownCharacter_C|SetIsShopOpen? (Variables|Default|GetTopDownCharRef) false)
  (Pawn|Components|CharacterMovement|SetMovementMode (Variables|/Script/Engine.Character|GetCharacterMovement (Variables|Default|GetTopDownCharRef)) "MOVE_Walking" 0)
  (if (Variables|/Game/InventorySystem/Blueprints/BP_Inventory.BP_Inventory_C|GetisVisible? (Variables|/Game/TopDownBP/Blueprints/TopDownCharacter.TopDownCharacter_C|GetInventoryRef (Variables|Default|GetTopDownCharRef)))
    (Default|HideInventory (Variables|/Game/TopDownBP/Blueprints/TopDownCharacter.TopDownCharacter_C|GetInventoryRef (Variables|Default|GetTopDownCharRef)))
    (Default|ShowInventory (Variables|/Game/TopDownBP/Blueprints/TopDownCharacter.TopDownCharacter_C|GetInventoryRef (Variables|Default|GetTopDownCharRef))))
  (Widget|RemovefromParent (Variables|Default|GetShopWidget))
  (Variables|Default|SetShopWidget 0)
  (Widget|SetIsEnabled (Variables|/Game/InventorySystem/Blueprints/BP_Inventory.BP_Inventory_C|GetInventoryWidget (Variables|/Game/TopDownBP/Blueprints/TopDownCharacter.TopDownCharacter_C|GetInventoryRef (Variables|Default|GetTopDownCharRef))) true)
  (Utilities|FlowControl|DoOnce false) ; enters at Reset
)

(fn ConstructionScript)